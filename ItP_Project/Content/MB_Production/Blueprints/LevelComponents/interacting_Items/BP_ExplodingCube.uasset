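; BP_ExplodingCube is a proximity-triggered explosive cube that damages its surroundings and destroys itself.
; On BeginPlay it creates a dynamic material instance for its static mesh.
; The first TriggerZone overlap latches a triggered flag and plays a timeline that lerps the base color between orange and red as a danger warning.
; When the timeline finishes, it applies radial damage around itself, prints a message and destroys the actor.
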(event `self.ReceiveBeginPlay`
  ; dynamic material from instance to modify it at runtime
  (bind _returnvalue (`PrimitiveComponent.CreateDynamicMaterialInstance` (`self.StaticMesh`) 0 null "None"))
  (set `self.DynamicMat` _returnvalue))

(event `self.TriggerZone.OnComponentBeginOverlap`
  (params (OverlappedComponent :type "PrimitiveComponent Object Reference") (OtherActor :type "Actor Object Reference") (OtherComp :type "PrimitiveComponent Object Reference") (OtherBodyIndex :type Integer) (bFromSweep :type Boolean) (SweepResult :type "HitResult Structure (by ref)"))
  ; on overlap, change status to is triggered
  (if (not (`self.isTRiggered`))
    (set `self.isTRiggered` true)
    ; Flashing red to portray danger
    (bind (_direction _flashalpha) (`Timeline|FlashTimeLine`)
      (:`Update`
        (`MaterialInstanceDynamic.SetVectorParameterValue` (`self.DynamicMat`) "Base Color" (`KismetMathLibrary.LinearColorLerp` (struct :`R` 1.0 :`G` 0.123916 :`B` 0.000457 :`A` 1.0) (struct :`R` 1.0 :`B` 0.00988 :`A` 1.0) _flashalpha)))
      (:`Finished`
        ; Apply Radial damage
        (`GameplayStatics.ApplyRadialDamage` (`self.BaseDamage`) (`self.K2_GetActorLocation`) 1000.0 "/Script/Engine.DamageType" (`|MakeArray` self :!type "Actor Object Reference") null null)
        (`KismetSystemLibrary.PrintString` "Boom!")
        (`self.K2_DestroyActor`)))))

(fn `UserConstructionScript`)