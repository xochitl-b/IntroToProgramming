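; BP_InvisibleWall is a level blocker that removes itself once all target cubes in its section are destroyed.
; On BeginPlay it finds every BP_TargetCube carrying its SectionTag, binds to each cube's destroyed event and counts them.
; Each destruction decrements the counter, and the wall destroys itself when the count reaches zero or below.
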(event `self.ReceiveBeginPlay`
  (bind _outactors (`GameplayStatics.GetAllActorsOfClassWithTag` "/Game/MB_Production/Blueprints/LevelComponents/LevelProps/BP_TargetCube.BP_TargetCube_C" (`self.SectionTag`)))
  (for _array_element _outactors
    (add `/Game/MB_Production/Blueprints/LevelComponents/LevelProps/BP_TargetCube.OnTargetDestroyed` _array_element (delegate `DecrTargetCounter`))
    (set `self.TargetCount` (+ (`self.TargetCount`) 1))))

(event `DecrTargetCounter`
  (bind _output_get (set `self.TargetCount` (- (`self.TargetCount`) 1)))
  (if (<= _output_get 0)
    (`self.K2_DestroyActor`)))

(fn `UserConstructionScript`)