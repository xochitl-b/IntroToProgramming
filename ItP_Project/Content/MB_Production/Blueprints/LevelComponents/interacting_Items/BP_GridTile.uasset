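; BP_GridTile is a grid tile that can be flagged as a hidden explosive hazard through WillExplode.
; On begin play it creates a dynamic material for its cube, and explosive tiles show orange-red for a few seconds before turning cyan, revealing the pattern briefly.
; When something overlaps the ExplosionZone of an explosive tile, it applies full radial damage around itself, prints a debug message, and destroys itself after a short delay.
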(event `self.ReceiveBeginPlay`
  (bind _returnvalue (`PrimitiveComponent.CreateDynamicMaterialInstance` (`self.Cube`) 0 null "None"))
  (set `self.TileMaterial` _returnvalue)
  (`self.ShowPattern`))

(event `ShowPattern`
  (if (`self.WillExplode`)
    (`MaterialInstanceDynamic.SetVectorParameterValue` (`self.TileMaterial`) "Base Color" (struct :`R` 1.0 :`G` 0.028332 :`B` 0.00023 :`A` 1.0))
    (`KismetSystemLibrary.Delay` 5.0)
    (`MaterialInstanceDynamic.SetVectorParameterValue` (`self.TileMaterial`) "Base Color" (struct :`R` 0.046665 :`G` 0.760525 :`B` 1.0 :`A` 1.0))))

(event `self.ExplosionZone.OnComponentBeginOverlap`
  (params (OverlappedComponent :type "PrimitiveComponent Object Reference") (OtherActor :type "Actor Object Reference") (OtherComp :type "PrimitiveComponent Object Reference") (OtherBodyIndex :type Integer) (bFromSweep :type Boolean) (SweepResult :type "HitResult Structure (by ref)"))
  (if (`self.WillExplode`)
    ; Apply Radial damage
    (`GameplayStatics.ApplyRadialDamage` 80.0 (`self.K2_GetActorLocation`) 400.0 "/Script/Engine.DamageType" (`|MakeArray` self :!type "Actor Object Reference") null null true)
    (`KismetSystemLibrary.PrintString` "Boom!")
    (`KismetSystemLibrary.Delay` 1.0)
    (`self.K2_DestroyActor`)))

(fn `UserConstructionScript`)