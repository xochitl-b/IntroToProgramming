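; BP_AmmoPickup is a pickup that adds ammo to the first-person shooter character's current weapon.
; When that character overlaps the collision component, it reads the current weapon class from the character's inventory and finds an instance with GetActorOfClass.
; It adds the pickup amount to that weapon's ammo, clamped to its maximum capacity, then destroys itself.
; The weapon lookup searches the world by class rather than using a reference held by the character.
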(event `self.Ammo_box_collision.OnComponentBeginOverlap`
  (params (OverlappedComponent :type "PrimitiveComponent Object Reference") (OtherActor :type "Actor Object Reference") (OtherComp :type "PrimitiveComponent Object Reference") (OtherBodyIndex :type Integer) (bFromSweep :type Boolean) (SweepResult :type "HitResult Structure (by ref)"))
  (bind _asbp_first_person_shooter_character (cast `/Game/MB_Production/Blueprints/BP_FirstPersonShooterCharacter` OtherActor))
  (bind _returnvalue (`GameplayStatics.GetActorOfClass` (`|GetArrayItem` (`/Game/MB_Production/Blueprints/BP_FirstPersonShooterCharacter.WeaponInventory` _asbp_first_person_shooter_character) (`/Game/MB_Production/Blueprints/BP_FirstPersonShooterCharacter.CurrentWeaponIndex` _asbp_first_person_shooter_character))))
  (set `/Game/MB_Production/Blueprints/Weapons/BP_weapon.CurrentAmmo` (`KismetMathLibrary.Clamp` (+ (`/Game/MB_Production/Blueprints/Weapons/BP_weapon.CurrentAmmo` _returnvalue) (`self.PickupAmmoAmount`)) 0 (`/Game/MB_Production/Blueprints/Weapons/BP_weapon.MaxAmmoCapacity` _returnvalue)) _returnvalue)
  (`self.K2_DestroyActor`))

(fn `UserConstructionScript`)