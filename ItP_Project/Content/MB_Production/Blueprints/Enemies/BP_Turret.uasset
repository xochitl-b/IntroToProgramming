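; BP_Turret is an enemy turret that tracks and shoots the first-person player, and prints a win message when destroyed.
; Each PawnSensing sighting turns it toward the player, then fires its child-actor gun from BulletStart.
; Aiming uses interpolated look-at rotation, split into actor yaw and clamped head pitch.
; Damage lowers integer health, printing what remains until zero destroys the actor.
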(event `self.ReceiveBeginPlay`
  (bind _asbp_turret_gun (cast `/Game/MB_Production/Blueprints/Weapons/BP_TurretGun` (`ChildActorComponent.ChildActor` (`self.TurretGun`))))
  (set `self.GunBp` _asbp_turret_gun))

(event `self.PawnSensing.OnSeePawn`
  (params (Pawn :type "Pawn Object Reference"))
  (bind _gunbp (`self.GunBp`))
  (bind _bulletstart (`self.BulletStart`))
  (bind _asbp_first_person_shooter_character (cast `/Game/MB_Production/Blueprints/BP_FirstPersonShooterCharacter` Pawn))
  (`self.TargetPlayer` _asbp_first_person_shooter_character)
  (`/Engine/EditorBlueprintResources/StandardMacros.IsValid` _gunbp
    (:`Is Valid`
      (`/Game/MB_Production/Blueprints/Weapons/BP_weapon.Shoot` _gunbp (`SceneComponent.K2_GetComponentLocation` _bulletstart) (`SceneComponent.GetForwardVector` _bulletstart))
      (`KismetSystemLibrary.PrintString` "Shooting"))))

(event `self.ReceiveAnyDamage`
  (params (Damage :type "Float (single-precision)") (DamageType :type "DamageType Object Reference") (InstigatedBy :type "Controller Object Reference") (DamageCauser :type "Actor Object Reference"))
  (bind _output_get (set `self.currentHealth` (`KismetMathLibrary.FTrunc` (- (`self.currentHealth`) Damage))))
  (if (<= _output_get 0)
    (`self.K2_DestroyActor`)
    (`KismetSystemLibrary.PrintString` "Dead")
    (`KismetSystemLibrary.PrintString` "You Won!")
    (else
      (`KismetSystemLibrary.PrintText` (`KismetTextLibrary.Conv_IntToText` (`self.currentHealth`))))))

(fn `TargetPlayer`
  (params (Player :type "Actor Object Reference"))
  (bind _head (`self.Head`))
  (bind (_returnvalue_roll _returnvalue_pitch _returnvalue_yaw) (`KismetMathLibrary.BreakRotator` (`KismetMathLibrary.RInterpTo` (`SceneComponent.K2_GetComponentRotation` _head) (`KismetMathLibrary.FindLookAtRotation` (`SceneComponent.K2_GetComponentLocation` _head) (`self.K2_GetActorLocation` Player)) (`GameplayStatics.GetWorldDeltaSeconds`) (`self.RotationSpeed`))))
  (`SceneComponent.K2_SetRelativeRotation` (`self.Head`) (`KismetMathLibrary.MakeRotator` 0.0 (`KismetMathLibrary.FClamp` _returnvalue_pitch -20.0 20.0)) false false)
  (`self.K2_SetActorRotation` (`KismetMathLibrary.MakeRotator` 0.0 0.0 _returnvalue_yaw)))

(fn `UserConstructionScript`)