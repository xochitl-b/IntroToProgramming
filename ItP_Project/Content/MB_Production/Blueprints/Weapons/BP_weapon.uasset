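; BP_weapon is a hitscan weapon Blueprint whose Shoot function fires one or more line traces from a given origin and direction.
; Multi-shot fire randomizes each trace within a spread cone, and a timer gates the fire rate through CanShoot.
; Movable physics-simulating hits receive a Damage-scaled impulse along the aim direction, while other hits take damage instead.
; Debug trace lines and print strings are left on.
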(event `ShootTimerExpired`
  (set `self.canShoot` true))

(fn `Shoot`
  (params (OriginLocation :type "Vector Structure") (ForwardVector :type "Vector Structure"))
  (if (`self.canShoot`)
    ; Loop to allow multiple shots
    (for _ (range (`self.shotCount`))
      (set `self.canShoot` false)
      (`KismetSystemLibrary.K2_SetTimerDelegate` (`|CreateDelegate` :!event `ShootTimerExpired`) (`self.FireDelay`))
      (bind _outhit (`KismetSystemLibrary.LineTraceSingle` :`Start` OriginLocation :`End` (+ OriginLocation (* (select `bool` (> (`self.shotCount`) 1) :`false` ForwardVector :`true` (`KismetMathLibrary.RandomUnitVectorInConeInDegrees` ForwardVector (`self.ShotSpread`))) (`self.Range`))) :`TraceChannel` "TraceTypeQuery1" :`DrawDebugType` "ForDuration" :`DrawTime` 1.0))
      (`/Engine/EditorBlueprintResources/StandardMacros.IsValid` (`.HitComponent` (`GameplayStatics.BreakHitResult` _outhit))
        (:`Is Valid`
          (if (and (`|EnumEquality` (`SceneComponent.Mobility` (`.HitComponent` (`GameplayStatics.BreakHitResult` _outhit))) "Movable") (`SceneComponent.IsSimulatingPhysics` (`.HitComponent` (`GameplayStatics.BreakHitResult` _outhit)) "None"))
            (`PrimitiveComponent.AddImpulseAtLocation` (`.HitComponent` (`GameplayStatics.BreakHitResult` _outhit)) (* ForwardVector (`self.Damage`)) (`.Location` (`GameplayStatics.BreakHitResult` _outhit)) "None")
            (`KismetSystemLibrary.PrintString` "It's shooting")
            (else
              (`GameplayStatics.ApplyDamage` (`.HitActor` (`GameplayStatics.BreakHitResult` _outhit)) (`self.Damage`))
              (`KismetSystemLibrary.PrintString` "Applying damage"))))))))

(fn `UserConstructionScript`)