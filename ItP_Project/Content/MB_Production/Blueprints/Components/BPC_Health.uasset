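; Actor component that gives its owning actor a health pool reduced by incoming damage.
; On BeginPlay it fills Health to MaxHealth and binds to the owner's OnTakeAnyDamage event.
; Each hit subtracts the damage, clamps Health between zero and the maximum, then broadcasts the new value through the OnHealthChanged dispatcher.
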(event `self.ReceiveBeginPlay`
  (set `self.Health` (`self.maxHealth`))
  (add `Actor.OnTakeAnyDamage` (`self.GetOwner`) (delegate `onDamageTaken`)))

(event `onDamageTaken`
  (params (DamagedActor :type "Actor Object Reference") (Damage :type "Float (single-precision)") (DamageType :type "DamageType Object Reference") (InstigatedBy :type "Controller Object Reference") (DamageCauser :type "Actor Object Reference"))
  (bind _output_get (set `self.Health` (`KismetMathLibrary.FClamp` (- (`self.Health`) Damage) 0.0 (`self.maxHealth`))))
  (`self.OnHealthChanged` _output_get))